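; BP_WidgetEvent is an interactable actor that shows a book widget filled with text from its description variable.
; It creates the book and interact-prompt widgets on BeginPlay, then hides them and disables its input.
; The player character entering the sphere shows the prompt and enables input; leaving removes both widgets and disables it.
; The E key uses a FlipFlop to swap between book and prompt, and leaving the sphere does not reset it.
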(event OnComponentBeginOverlap(Sphere)
  (params (OverlappedComponent :type Primitive%20Component%20Object%20Reference) (OtherActor :type Actor%20Object%20Reference) (OtherComp :type Primitive%20Component%20Object%20Reference) (OtherBodyIndex :type Integer) (bFromSweep :type Boolean) (SweepResult :type Hit%20Result%20Structure%20%28by%20ref%29))
  (Utilities|Casting|CastToBP_ThirdPersonCharacterCustom OtherActor)
  (UserInterface|Viewport|AddtoViewport (stale EventBeginPlay _returnvalue_2) 0)
  (Input|EnableInput (Game|GetPlayerController 0)))

(event OnComponentEndOverlap(Sphere)
  (params (OverlappedComponent :type Primitive%20Component%20Object%20Reference) (OtherActor :type Actor%20Object%20Reference) (OtherComp :type Primitive%20Component%20Object%20Reference) (OtherBodyIndex :type Integer))
  (Utilities|Casting|CastToBP_ThirdPersonCharacterCustom OtherActor)
  (Widget|RemovefromParent (stale EventBeginPlay _returnvalue_2))
  (Input|DisableInput (Game|GetPlayerController 0)))

(event EventBeginPlay
  (bind _returnvalue (UserInterface|CreateWidget "/Game/Widgets/W_Book.W_Book_C"))
  (Variables|/Script/UMG.TextBlock|SetText (Variables|/Game/Widgets/W_Book.W_Book_C|GetTextBlock_0 _returnvalue) (Variables|Default|GetDescriptionVariable))
  (bind _returnvalue_2 (UserInterface|CreateWidget "/Game/Widgets/InteractWidget.InteractWidget_C"))
  (Widget|RemovefromParent _returnvalue_2)
  (Input|DisableInput (Game|GetPlayerController 0)))

(event Input|KeyboardEvents|E
  (params (Key :type Key%20Structure :default "None"))
  (:Pressed
    (Utilities|FlowControl|FlipFlop
      (:A
        (UserInterface|Viewport|AddtoViewport (stale EventBeginPlay _returnvalue) 0)
        (Widget|RemovefromParent (stale EventBeginPlay _returnvalue_2)))
      (:B
        (Widget|RemovefromParent (stale EventBeginPlay _returnvalue))
        (UserInterface|Viewport|AddtoViewport (stale EventBeginPlay _returnvalue_2) 0)))))

(fn ConstructionScript)
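; BP_UIPickUp is an actor that shows a floating pickup label through a widget component.
; On BeginPlay it creates a W_UIPickUp widget, assigns it to the component and sets the item name text to the actor's own display name.
; A self-calling event on a short delay, used in place of Tick, keeps turning the widget toward the player camera.
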(event Custom|RotateTowardsPlayer
  (Transformation|SetWorldRotation (Variables|Default|GetWidget) (Math|Rotator|FindLookatRotation (Transformation|GetWorldLocation (Variables|Default|GetWidget)) (Transformation|GetWorldLocation (Variables|/Script/Engine.PlayerCameraManager|GetTransformComponent (Game|GetPlayerCameraManager 0)))) false false)
  (Utilities|FlowControl|Delay 0.1)
  (CallFunction|RotateTowardsPlayer))

(event EventBeginPlay
  (bind _returnvalue (UserInterface|CreateWidget "/Game/Widgets/W_UIPickUp.W_UIPickUp_C"))
  (UserInterface|SetWidget (Variables|Default|GetWidget) _returnvalue)
  (Variables|/Script/UMG.TextBlock|SetText (Variables|/Game/Widgets/W_UIPickUp.W_UIPickUp_C|GetItemName _returnvalue) (Utilities|Text|ToText(String) (Utilities|GetDisplayName self)))
  (CallFunction|RotateTowardsPlayer))

(event Collision|EventActorBeginOverlap
  (params (OtherActor :type Actor%20Object%20Reference)))

(event EventTick
  (params (DeltaSeconds :type Float%20%28single-precision%29)))

(fn ConstructionScript)
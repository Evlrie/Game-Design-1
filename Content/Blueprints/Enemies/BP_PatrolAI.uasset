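; BP_PatrolAI is an enemy character that patrols between tagged patrol point actors at a randomised walk speed.
; On BeginPlay it gathers and shuffles the points, then loops AI MoveTo through them with a short pause, reshuffling after each full round.
; A separate GoToDestination event repeatedly moves to the player, but nothing in this file calls it.
; A failed move only prints a message, ending that loop.
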(event Custom|GoToPatrolPoint
  ;[1 0.4983 0.4983] Patrol
  (AI|AIMoveTo self (Transformation|GetActorLocation (Utilities|Array|Get(acopy) (stale EventBeginPlay _outactors) (Variables|Default|GetCurrentPatrolPoint))) 0 5.0 false
    (:OnSuccess
      (Development|PrintString "Arrived at Destination")
      (bind _result (Math|Integer|IncrementInt (Variables|Default|GetCurrentPatrolPoint))
        (:%20%20
          (if (>= _result (Utilities|Array|Length (stale EventBeginPlay _outactors)))
            (Variables|Default|SetCurrentPatrolPoint 0)
            (Utilities|Array|Shuffle (stale EventBeginPlay _outactors)))
          (Utilities|FlowControl|Delay 1.0)
          (CallFunction|GotoPatrolPoint))))
    (:OnFail
      (Development|PrintString "Failed to get to Destination"))))

(event Custom|GoToDestination
  ;[0.4583 0.8136 1] Go To Player
  (AI|AIMoveTo self "0, 0, 0" (Game|GetPlayerCharacter 0) 5.0 false
    (:OnSuccess
      (Development|PrintString "Arrived at Destination")
      (Utilities|FlowControl|Delay 1.0)
      (CallFunction|GotoDestination))
    (:OnFail
      (Development|PrintString "Failed to get to Destination"))))

(event EventBeginPlay
  ;[0.9942 0.6145 1] Begin Play
  (bind _outactors (Actor|GetAllActorsOfClasswithTag "/Script/Engine.Actor" "PatrolPointEnv"))
  (Development|PrintString (Utilities|String|Append "There are " (Utilities|String|ToString(Integer) (Utilities|Array|Length _outactors)) "append links"))
  (Utilities|Array|Shuffle _outactors)
  (Variables|/Script/Engine.CharacterMovementComponent|SetMaxWalkSpeed (Variables|Character|GetCharacterMovement) (Math|Conversions|ToFloat(Integer) (* (Math|Random|RandomIntegerinRange 8 12) 50)))
  (CallFunction|GotoPatrolPoint))

(fn ConstructionScript)
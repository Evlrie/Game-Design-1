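; BP_FallingCeiling is a trap ceiling that, once activated (noted as a pressure plate trigger), plays a falling sound and moves up and down repeatedly.
; A timeline lerps the Ceiling between Start and End component locations, and a FlipFlop on completion alternates reverse and forward playback to loop endlessly.
; Overlapping its Box sends the player character back to the last checkpoint via LoadCheckpoint.
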(event OnComponentBeginOverlap(Box)
  (params (OverlappedComponent :type Primitive%20Component%20Object%20Reference) (OtherActor :type Actor%20Object%20Reference) (OtherComp :type Primitive%20Component%20Object%20Reference) (OtherBodyIndex :type Integer) (bFromSweep :type Boolean) (SweepResult :type Hit%20Result%20Structure%20%28by%20ref%29))
  (bind _asbp_third_person_character_custom (Utilities|Casting|CastToBP_ThirdPersonCharacterCustom OtherActor))
  (Default|LoadCheckpoint _asbp_third_person_character_custom))

(event Custom|Activated
  (Audio|PlaySoundatLocation "/Game/Blueprints/Audio/Falling_Wall_2_Cue.Falling_Wall_2_Cue" (Transformation|GetWorldLocation (Variables|Default|GetCeiling)) "0, 0, 0" 1.0 1.0 0.0 0 0 0 0)
  (bind _floattrack (Timeline|Timeline Play)
    (:Update
      (Transformation|SetRelativeLocation (Variables|Default|GetCeiling) (Math|Vector|Lerp(Vector) (Variables|/Script/Engine.SceneComponent|GetRelativeLocation (Variables|Default|GetStart)) (Variables|/Script/Engine.SceneComponent|GetRelativeLocation (Variables|Default|GetEnd)) _floattrack) false false))
    (:Finished
      (Utilities|FlowControl|FlipFlop ; Loops the ceiling falling
        (:A
          (Timeline|Timeline ReverseFromEnd))
        (:B
          (Timeline|Timeline Play))))))

(event EventBeginPlay)

(event Collision|EventActorBeginOverlap
  (params (OtherActor :type Actor%20Object%20Reference)))

(event EventTick
  (params (DeltaSeconds :type Float%20%28single-precision%29)))

(fn ConstructionScript)
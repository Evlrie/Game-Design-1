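; BP_FakePlate is a decoy pressure plate that springs a falling-ceiling trap when any actor overlaps it.
; The overlap prints panicked warnings urging the other plates to be activated, then calls Activated on a CeilingActivation reference to start the ceiling event.
; A Timeline then lerps the Cube between the Start and End component locations to animate the plate.
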(event EventBeginPlay)

(event EventTick
  (params (DeltaSeconds :type Float%20%28single-precision%29)))

(event Collision|EventActorBeginOverlap
  (params (OtherActor :type Actor%20Object%20Reference))
  (Development|PrintString "THE CEILING IS FALLING!!!" true true "(R=1.000000,G=0.070948,B=0.000000,A=1.000000)" 5.0)
  (Development|PrintString "Quick activate the other plates! Before we're mush!" true true "(R=1.000000,G=0.070360,B=0.000000,A=1.000000)" 5.0)
  (Default|Activated (Variables|Default|GetCeilingActivation))
  (bind _newtrack_0 (Timeline|Timeline Play)
    (:Update
      (Transformation|SetRelativeLocation (Variables|Default|GetCube) (Math|Vector|Lerp(Vector) (Variables|/Script/Engine.SceneComponent|GetRelativeLocation (Variables|Default|Getstart)) (Variables|/Script/Engine.SceneComponent|GetRelativeLocation (Variables|Default|GetEnd)) _newtrack_0) false false))))

(fn ConstructionScript)
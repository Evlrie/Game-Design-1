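; BP_MovingDoor is a door that opens once enough pressure switches are active at the same time.
; Activated and Deactivated events adjust an active switch count and compare it to PressureSwitchesNeeded to play or reverse a Timeline.
; The Timeline lerps the Sphere component between the Start and End relative locations, with a sound and message on opening.
; Overlapping the Box plays a banging sound and prints a hint.
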(event OnComponentBeginOverlap(Box)
  (params (OverlappedComponent :type Primitive%20Component%20Object%20Reference) (OtherActor :type Actor%20Object%20Reference) (OtherComp :type Primitive%20Component%20Object%20Reference) (OtherBodyIndex :type Integer) (bFromSweep :type Boolean) (SweepResult :type Hit%20Result%20Structure%20%28by%20ref%29))
  ;[1 0.8411 0.5051] Gives hint on how to open door
  (Audio|PlaySoundatLocation "/Game/Blueprints/Audio/FranticBang_Cue.FranticBang_Cue" (Transformation|GetWorldLocation (Variables|Default|GetBox)) "0, 0, 0" 1.0 1.0 0.0 0 0 0 0)
  (Development|PrintString "Looks like a door. There has to be a way to open it." true true "(R=0.200758,G=1.000000,B=0.000000,A=1.000000)" 5.0))

(event Custom|Activated
  ;[1 0.5167 0.7485] Switches needed to open door code
  (Math|Integer|IncrementInt (Variables|Default|GetActiveSwitches)
    (:%20%20
      (if (>= (Variables|Default|GetActiveSwitches) (Variables|Default|GetPressureSwitchesNeeded))
        (Development|PrintString "Nice! The door opened!" true true "(R=0.034797,G=1.000000,B=0.000000,A=1.000000)" 4.0)
        (Audio|PlaySoundatLocation "/Game/Blueprints/Audio/Falling_platform_Cue.Falling_platform_Cue" (Transformation|GetWorldLocation (Variables|Default|GetDefaultSceneRoot)) "0, 0, 0" 1.0 1.0 0.0 0 0 0 0)
        (bind _newtrack_0 (Timeline|Timeline Play)
          (:Update
            (Transformation|SetRelativeLocation (Variables|Default|GetSphere) (Math|Vector|Lerp(Vector) (Variables|/Script/Engine.SceneComponent|GetRelativeLocation (Variables|Default|GetStart)) (Variables|/Script/Engine.SceneComponent|GetRelativeLocation (Variables|Default|GetEnd)) _newtrack_0) false false)))
        (else
          (Development|PrintString "Hmm...I think we need to activate more?" true true "(R=1.000000,G=0.048611,B=0.078026,A=1.000000)" 3.0)
          (Timeline|Timeline Reverse))))))

(event Custom|Deactivated
  ;[1 0.5167 0.7485] Switches needed to open door code
  (Math|Integer|DecrementInt (Variables|Default|GetActiveSwitches)
    (:%20%20
      (if (>= (Variables|Default|GetActiveSwitches) (Variables|Default|GetPressureSwitchesNeeded))
        (bind _newtrack_0 (Timeline|Timeline Play)
          (:Update
            (Transformation|SetRelativeLocation (Variables|Default|GetSphere) (Math|Vector|Lerp(Vector) (Variables|/Script/Engine.SceneComponent|GetRelativeLocation (Variables|Default|GetStart)) (Variables|/Script/Engine.SceneComponent|GetRelativeLocation (Variables|Default|GetEnd)) _newtrack_0) false false)))
        (else
          (Timeline|Timeline Reverse))))))

(event EventBeginPlay)

(event Collision|EventActorBeginOverlap
  (params (OtherActor :type Actor%20Object%20Reference)))

(event EventTick
  (params (DeltaSeconds :type Float%20%28single-precision%29)))

(fn ConstructionScript)
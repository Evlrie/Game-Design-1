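; BP_DeathWall is a moving wall trap that sends the player back to a checkpoint on contact.
; The Activated event, noted as pressure-plate triggered, starts a Timeline that lerps the DeathWall between the Start and End relative locations.
; A FlipFlop on Timeline completion alternates reverse and forward playback, so the wall keeps cycling once activated.
; Box overlap with BP_ThirdPersonCharacterCustom calls its LoadCheckpoint.
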(event OnComponentBeginOverlap(Box)
  (params (OverlappedComponent :type Primitive%20Component%20Object%20Reference) (OtherActor :type Actor%20Object%20Reference) (OtherComp :type Primitive%20Component%20Object%20Reference) (OtherBodyIndex :type Integer) (bFromSweep :type Boolean) (SweepResult :type Hit%20Result%20Structure%20%28by%20ref%29))
  ;[1 0.734 0.1895] Kills player when hit and respawns at checkpoint
  (bind _asbp_third_person_character_custom (Utilities|Casting|CastToBP_ThirdPersonCharacterCustom OtherActor))
  (Default|LoadCheckpoint _asbp_third_person_character_custom))

(event Custom|Activated
  ;[1 0.1875 0.1908] Moves platform when trap is activated
  (bind _floattrack (Timeline|Timeline PlayFromStart)
    (:Update
      (Transformation|SetRelativeLocation (Variables|Default|GetDeathWall) (Math|Vector|Lerp(Vector) (Variables|/Script/Engine.SceneComponent|GetRelativeLocation (Variables|Default|GetStart)) (Variables|/Script/Engine.SceneComponent|GetRelativeLocation (Variables|Default|GetEnd)) _floattrack) false false))
    (:Finished
      (Utilities|FlowControl|FlipFlop
        (:A
          (Timeline|Timeline ReverseFromEnd))
        (:B
          (Timeline|Timeline PlayFromStart))))))

(event Collision|EventActorBeginOverlap
  (params (OtherActor :type Actor%20Object%20Reference)))

(event EventTick
  (params (DeltaSeconds :type Float%20%28single-precision%29)))

(fn ConstructionScript)
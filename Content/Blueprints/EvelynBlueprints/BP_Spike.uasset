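; BP_Spike is a moving spike hazard that sends the player back to a checkpoint on contact.
; From BeginPlay, a Timeline lerps Spike1's relative location between the Start and End components.
; Each time the Timeline finishes, a short delay and a FlipFlop alternate reverse and forward playback, looping the motion indefinitely.
; Overlapping the Box calls LoadCheckpoint on the BP_ThirdPersonCharacterCustom that touched it, ignoring other actors.
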(event OnComponentBeginOverlap(Box)
  (params (OverlappedComponent :type Primitive%20Component%20Object%20Reference) (OtherActor :type Actor%20Object%20Reference) (OtherComp :type Primitive%20Component%20Object%20Reference) (OtherBodyIndex :type Integer) (bFromSweep :type Boolean) (SweepResult :type Hit%20Result%20Structure%20%28by%20ref%29))
  (bind _asbp_third_person_character_custom (Utilities|Casting|CastToBP_ThirdPersonCharacterCustom OtherActor))
  (Default|LoadCheckpoint _asbp_third_person_character_custom))

(event EventBeginPlay
  (bind _newtrack_0 (Timeline|Timeline PlayFromStart)
    (:Update
      (Transformation|SetRelativeLocation (Variables|Default|GetSpike1) (Math|Vector|Lerp(Vector) (Variables|/Script/Engine.SceneComponent|GetRelativeLocation (Variables|Default|GetStart)) (Variables|/Script/Engine.SceneComponent|GetRelativeLocation (Variables|Default|Getend)) _newtrack_0) false false))
    (:Finished
      (Utilities|FlowControl|Delay 0.2)
      (Utilities|FlowControl|FlipFlop
        (:A
          (Timeline|Timeline ReverseFromEnd))
        (:B
          (Timeline|Timeline PlayFromStart))))))

(event Collision|EventActorBeginOverlap
  (params (OtherActor :type Actor%20Object%20Reference)))

(event EventTick
  (params (DeltaSeconds :type Float%20%28single-precision%29)))

(fn ConstructionScript)
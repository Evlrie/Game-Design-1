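; BP_SpikeTrap2 is a moving spike trap that sends the player back to a checkpoint on contact.
; From BeginPlay, the Movement timeline lerps Trap between the Beginning and End relative locations without sweep, and a FlipFlop on Finished alternates reverse and forward playback to loop it endlessly.
; When BP_ThirdPersonCharacterCustom begins overlapping Box, the trap calls that character's LoadCheckpoint.
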(event OnComponentBeginOverlap(Box)
  (params (OverlappedComponent :type Primitive%20Component%20Object%20Reference) (OtherActor :type Actor%20Object%20Reference) (OtherComp :type Primitive%20Component%20Object%20Reference) (OtherBodyIndex :type Integer) (bFromSweep :type Boolean) (SweepResult :type Hit%20Result%20Structure%20%28by%20ref%29))
  (bind _asbp_third_person_character_custom (Utilities|Casting|CastToBP_ThirdPersonCharacterCustom OtherActor))
  (Default|LoadCheckpoint _asbp_third_person_character_custom))

(event EventBeginPlay
  ;[1 0.4956 0.9947] Makes the Spike trap move
  (bind _newtrack_0 (Timeline|Movement PlayFromStart)
    (:Update
      (Transformation|SetRelativeLocation (Variables|Default|GetTrap) (Math|Vector|Lerp(Vector) (Variables|/Script/Engine.SceneComponent|GetRelativeLocation (Variables|Default|GetBeginning)) (Variables|/Script/Engine.SceneComponent|GetRelativeLocation (Variables|Default|GetEnd)) _newtrack_0) false false))
    (:Finished
      (Utilities|FlowControl|FlipFlop
        (:A
          (Timeline|Movement ReverseFromEnd))
        (:B
          (Timeline|Movement PlayFromStart))))))

(event Collision|EventActorBeginOverlap
  (params (OtherActor :type Actor%20Object%20Reference)))

(event EventTick
  (params (DeltaSeconds :type Float%20%28single-precision%29)))

(fn ConstructionScript)
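; BP_Treasure is a collectible pickup actor, presented to the player as a gold egg, that adds to the character's jewel tally.
; When its Sphere1 component is overlapped by BP_ThirdPersonCharacterCustom, it increments that character's JewelCount and prints the new total.
; It then plays the key sound cue at its location and destroys itself.
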(event OnComponentBeginOverlap(Sphere1)
  (params (OverlappedComponent :type Primitive%20Component%20Object%20Reference) (OtherActor :type Actor%20Object%20Reference) (OtherComp :type Primitive%20Component%20Object%20Reference) (OtherBodyIndex :type Integer) (bFromSweep :type Boolean) (SweepResult :type Hit%20Result%20Structure%20%28by%20ref%29))
  (bind _asbp_third_person_character_custom (Utilities|Casting|CastToBP_ThirdPersonCharacterCustom OtherActor))
  (Variables|/Game/Blueprints/BP_ThirdPersonCharacterCustom.BP_ThirdPersonCharacterCustom_C|SetJewelCount _asbp_third_person_character_custom (+ (Variables|/Game/Blueprints/BP_ThirdPersonCharacterCustom.BP_ThirdPersonCharacterCustom_C|GetJewelCount _asbp_third_person_character_custom) 1))
  (Development|PrintString (Utilities|String|Append "You have " (Utilities|String|ToString(Integer) (Variables|/Game/Blueprints/BP_ThirdPersonCharacterCustom.BP_ThirdPersonCharacterCustom_C|GetJewelCount _asbp_third_person_character_custom)) " gold eggs!"))
  (Audio|PlaySoundatLocation "/Game/Blueprints/Audio/key_Cue.key_Cue" (Transformation|GetWorldLocation (Variables|Default|GetDefaultSceneRoot)) "0, 0, 0" 1.0 1.0 0.0 0 0 0 0)
  (Actor|DestroyActor))

(event Collision|EventActorBeginOverlap
  (params (OtherActor :type Actor%20Object%20Reference)))

(event EventTick
  (params (DeltaSeconds :type Float%20%28single-precision%29)))

(fn ConstructionScript)
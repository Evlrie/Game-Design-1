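; BP_JewelKey is a collectible jewel pickup that adds to the player's special jewel count.
; When a BP_ThirdPersonCharacterCustom overlaps its Sphere1 component, it increments that character's JewelCount, prints pickup and total messages, then destroys itself.
; BeginPlay prints a debug message confirming the jewel exists, and the counter is stored on the character rather than the pickup.
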(event OnComponentBeginOverlap(Sphere1)
  (params (OverlappedComponent :type Primitive%20Component%20Object%20Reference) (OtherActor :type Actor%20Object%20Reference) (OtherComp :type Primitive%20Component%20Object%20Reference) (OtherBodyIndex :type Integer) (bFromSweep :type Boolean) (SweepResult :type Hit%20Result%20Structure%20%28by%20ref%29))
  (bind _asbp_third_person_character_custom (Utilities|Casting|CastToBP_ThirdPersonCharacterCustom OtherActor))
  (Development|PrintString "You picked up a special jewel...maybe you can use it somewhere!" true true "(R=0.067566,G=1.000000,B=0.000000,A=1.000000)" 5.0)
  (Variables|/Game/Blueprints/BP_ThirdPersonCharacterCustom.BP_ThirdPersonCharacterCustom_C|SetJewelCount _asbp_third_person_character_custom (+ (Variables|/Game/Blueprints/BP_ThirdPersonCharacterCustom.BP_ThirdPersonCharacterCustom_C|GetJewelCount _asbp_third_person_character_custom) 1))
  (Development|PrintString (Utilities|String|Append "You have " (Utilities|String|ToString(Integer) (Variables|/Game/Blueprints/BP_ThirdPersonCharacterCustom.BP_ThirdPersonCharacterCustom_C|GetJewelCount _asbp_third_person_character_custom)) " special jewels."))
  (Actor|DestroyActor))

(event EventBeginPlay
  (Development|PrintString "Jewel Key Exists" true true "(R=1.000000,G=0.443061,B=0.099081,A=1.000000)"))

(event Collision|EventActorBeginOverlap
  (params (OtherActor :type Actor%20Object%20Reference)))

(event EventTick
  (params (DeltaSeconds :type Float%20%28single-precision%29)))

(fn ConstructionScript)
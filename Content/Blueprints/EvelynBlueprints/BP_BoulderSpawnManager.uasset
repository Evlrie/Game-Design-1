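; Manager actor that spawns waves of boulders at every BP_BoulderSpawner in the level.
; On BeginPlay it gathers all spawners, then spawns a BP_Boulder at each one's root location and rotation, passing itself as that boulder's manager and counting it.
; RemoveBoulder decrements the live count and spawns a fresh set at all spawners once none remain.
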(event Custom|SpawnBoulder
  ;[1 0.5135 0.4703] Spawns boulder at the spawner
  (for _array_element (Variables|Default|GetSpawners)
    (bind _returnvalue (Game|SpawnActorfromClass "/Game/Blueprints/EvelynBlueprints/BP_Boulder.BP_Boulder_C" (Math|Transform|MakeTransform (.location (Transformation|GetWorldTransform (Variables|/Game/Blueprints/EvelynBlueprints/BP_BoulderSpawner.BP_BoulderSpawner_C|GetDefaultSceneRoot _array_element))) (.rotation (Transformation|GetWorldTransform (Variables|/Game/Blueprints/EvelynBlueprints/BP_BoulderSpawner.BP_BoulderSpawner_C|GetDefaultSceneRoot _array_element))) "1.000000,1.000000,1.000000") "Undefined" "MultiplyWithRoot" 0 0)) ; spawns boulder at location and rotation
    (Variables|/Game/Blueprints/EvelynBlueprints/BP_Boulder.BP_Boulder_C|SetBoulderManager _returnvalue self)
    (Math|Integer|IncrementInt (Variables|Default|GetCurrentBoulderTotal))))

(event Custom|RemoveBoulder
  (Math|Integer|DecrementInt (Variables|Default|GetCurrentBoulderTotal)
    (:%20%20
      (if (not (> (Variables|Default|GetCurrentBoulderTotal) 0))
        (CallFunction|SpawnBoulder)))))

(event EventBeginPlay
  (bind _outactors (Actor|GetAllActorsOfClass "/Game/Blueprints/EvelynBlueprints/BP_BoulderSpawner.BP_BoulderSpawner_C"))
  (Variables|Default|SetSpawners _outactors)
  (CallFunction|SpawnBoulder))

(fn ConstructionScript)
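; BP_Scythe is a scythe hazard that sends the player back to a checkpoint on contact.
; Tick calls Play on a timeline, whose track lerps the Handle's relative rotation between the rotations of the Start and End components to move the scythe.
; A Box overlap casts the other actor to BP_ThirdPersonCharacterCustom and calls LoadCheckpoint on it.
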(event OnComponentBeginOverlap(Box)
  (params (OverlappedComponent :type Primitive%20Component%20Object%20Reference) (OtherActor :type Actor%20Object%20Reference) (OtherComp :type Primitive%20Component%20Object%20Reference) (OtherBodyIndex :type Integer) (bFromSweep :type Boolean) (SweepResult :type Hit%20Result%20Structure%20%28by%20ref%29))
  (bind _asbp_third_person_character_custom (Utilities|Casting|CastToBP_ThirdPersonCharacterCustom OtherActor))
  (Default|LoadCheckpoint _asbp_third_person_character_custom))

(event EventBeginPlay)

(event Collision|EventActorBeginOverlap
  (params (OtherActor :type Actor%20Object%20Reference)))

(event EventTick
  (params (DeltaSeconds :type Float%20%28single-precision%29))
  (bind _newtrack_1 (Timeline|Timeline Play)
    (:Update
      (Transformation|SetRelativeRotation (Variables|Default|GetHandle) (Math|Rotator|Lerp(Rotator) (Variables|/Script/Engine.SceneComponent|GetRelativeRotation (Variables|Default|GetStart)) (Variables|/Script/Engine.SceneComponent|GetRelativeRotation (Variables|Default|GetEnd)) _newtrack_1) false false))))

(fn ConstructionScript)